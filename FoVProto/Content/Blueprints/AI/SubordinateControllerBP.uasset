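; AI controller for subordinate characters that turns perception updates into blackboard state.
; Sensed FoVCharacters are added to, and lost ones removed from, the CharacterList object stored under the SeenCharacters key.
; When the updated actor is the blackboard Target, SeesTarget mirrors whether it is sensed.
; The node that would run Subordinate_BT is unconnected, so this graph never starts the behavior tree.
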(event OnTargetPerceptionUpdated(perception)
  (params (Actor :type Actor%20Object%20Reference) (Stimulus :type AI%20Stimulus%20Structure))
  (bind _returnvalue (AI|GetBlackboard 0))
  (bind _asfo_vcharacter (Utilities|Casting|CastToFoVCharacter Actor))
  (bind _ascharacter_list (Utilities|Casting|CastToCharacterList (AI|Components|Blackboard|GetValueasObject _returnvalue (Utilities|Name|MakeLiteralName "SeenCharacters"))))
  (bind _returnvalue_2 (Class|CharacterList|GetCharacters _ascharacter_list))
  (if (.bsuccessfullysensed Stimulus)
    (Utilities|Array|Add _returnvalue_2 _asfo_vcharacter)
    (else
      (Utilities|Array|RemoveItem _returnvalue_2 _asfo_vcharacter)))
  (if (== _asfo_vcharacter (AI|Components|Blackboard|GetValueasObject _returnvalue (Utilities|Name|MakeLiteralName "Target")))
    (AI|Components|Blackboard|SetValueasBool _returnvalue (Utilities|Name|MakeLiteralName "SeesTarget") (.bsuccessfullysensed Stimulus))))

(event EventBeginPlay)

(event EventTick
  (params (DeltaSeconds :type Float%20%28single-precision%29)))

(fn ConstructionScript)
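; FoVGameModeBP is a game mode that spawns an actor at player spawn points on BeginPlay for surplus players.
; It loops over the player count and, only for indices at or beyond the spawn count, reuses spawns offset by that count, adjusting for collision.
; The direct spawn for indices within range is disconnected, so those players get nothing spawned here.
; Tick and the construction script are empty.
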(event EventBeginPlay
  (bind _returnvalue (Class|GameModeBase|GetNumPlayers))
  (for _index (range 0 (- _returnvalue 1))
    (bind _returnvalue_2 (Class|FoVGameMode|GetPlayerSpawns))
    (if (>= _index (Utilities|Array|Length _returnvalue_2))
      (Game|SpawnActorfromClass 0 (Transformation|GetActorTransform (Utilities|Array|Get(acopy) _returnvalue_2 (- _index (Utilities|Array|Length _returnvalue_2)))) "AdjustIfPossibleButDontSpawnIfColliding" 0))))

(event EventTick
  (params (DeltaSeconds :type Float%20%28single-precision%29)))

(fn ConstructionScript)